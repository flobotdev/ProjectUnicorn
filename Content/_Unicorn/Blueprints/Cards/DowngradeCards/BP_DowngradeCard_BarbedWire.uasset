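; BP_DowngradeCard_BarbedWire is the Barbed Wire downgrade card, which forces its card effect on the owner when unicorns move in their stable.
; On entering a stable it binds to the CardManager's stable-change event.
; Any Baby, Basic or Magical Unicorn change for the owning player, without checking the Removed flag, invokes the non-optional effect.
; It then listens for that effect's execution, unbinds and calls NextPhase.
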(event Custom|OnPlayerStableChanged
  (params (PlayerIndex :type Integer) (Card :type Unicorn%20Card%20Actor%20Object%20Reference) (bRemoved :type Boolean))
  (if (== (Variables|Default|GetCurrentOwningPlayer) PlayerIndex)
    (switch Utilities|FlowControl|Switch|SwitchonECardType (.cardtype (Class|UnicornCardActor|GetCardInfo Card))
      (:MagicalUnicorn
        _)
      (:BasicUnicorn
        _)
      (:BabyUnicorn
        _))
    (Class|UnicornCardGameManager|InvokeEffect (Variables|Default|GetCardManager) (Variables|Default|GetCurrentOwningPlayer) (Utilities|Struct|BreakUnicornCardInfo (Variables|Default|GetCardInfo)) false)
    (EventDispatchers|BindEventtoOnEffectEventExecuted (Variables|Default|GetCardManager) (EventDispatchers|CreateEvent :!event Custom|OnEffectExecuted))))

(event Custom|OnEffectExecuted
  (params (Effect :type EEffectWord%20Enum :default "None") (PlayerIndex :type Integer) (bOptional :type Boolean))
  (if (Utilities|Enum|Equal(Enum) Effect (Utilities|Struct|BreakUnicornCardInfo (Variables|Default|GetCardInfo)))
    (EventDispatchers|UnbindEventfromOnEffectEventExecuted (Variables|Default|GetCardManager) (EventDispatchers|CreateEvent :!event Custom|OnEffectExecuted))
    (Class|UnicornCardGameManager|NextPhase (Variables|Default|GetCardManager))))

(event EventBeginPlay
  (|CallParentFunction) ; This node is disabled and will not be called.\nDrag off pins to build functionality.
)

(event Collision|EventActorBeginOverlap
  (params (OtherActor :type Actor%20Object%20Reference))
  (|CallParentFunction OtherActor) ; This node is disabled and will not be called.\nDrag off pins to build functionality.
)

(event EventTick
  (params (DeltaSeconds :type Float%20%28single-precision%29))
  (|CallParentFunction DeltaSeconds) ; This node is disabled and will not be called.\nDrag off pins to build functionality.
)

(event EventOnEnterStable
  (Variables|Default|GetCardManager
    (:then
      (EventDispatchers|BindEventtoOnPlayerStableChanged (Variables|Default|GetCardManager) (EventDispatchers|CreateEvent :!event Custom|OnPlayerStableChanged)))
    (:else)))

(fn ConstructionScript
  (|CallParentFunction))