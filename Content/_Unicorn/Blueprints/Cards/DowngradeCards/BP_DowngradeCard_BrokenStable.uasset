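; Broken Stable downgrade card that blocks its owning player's Upgrade cards from entering a stable while it is in play.
; On entering the stable, it disables Upgrade cards in that hand, records them and subscribes to CardManager hand changes.
; Cards added to the hand trigger a fresh scan, while recorded cards that leave it are re-enabled.
; On leaving, it re-enables recorded cards still in hand and unsubscribes.
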(event Custom|OnPlayerHandChanged
  (params (PlayerIndex :type Integer) (Card :type Unicorn%20Card%20Actor%20Object%20Reference) (bRemoved :type Boolean))
  (if (== PlayerIndex (Variables|Default|GetCurrentOwningPlayer))
    (if bRemoved
      (if (Utilities|Array|ContainsItem (Variables|Default|GetListOfAffectedCards) Card)
        (Class|UnicornCardActor|SetCanEnterStable Card true)
        (Utilities|Array|RemoveItem (Variables|Default|GetListOfAffectedCards) Card))
      (else
        (CallFunction|DisableCards)))))

(event EventOnLeaveStable
  (|CallParentFunction)
  (CallFunction|Revert)
  (EventDispatchers|UnbindEventfromOnPlayerHandChanged (Variables|Default|GetCardManager) (EventDispatchers|CreateEvent :!event Custom|OnPlayerHandChanged)))

(event EventOnEnterStable
  (CallFunction|DisableCards)
  (EventDispatchers|BindEventtoOnPlayerHandChanged (Variables|Default|GetCardManager) (EventDispatchers|CreateEvent :!event Custom|OnPlayerHandChanged)))

(fn ConstructionScript
  (|CallParentFunction))

(fn Revert
  (bind _cardmanager (Variables|Default|GetCardManager)
    (:then
      (LocalVariables|SetHand (Class|UnicornCardGameManager|GetPlayerHand _cardmanager (Variables|Default|GetCurrentOwningPlayer)))
      (for _array_element (Variables|Default|GetListOfAffectedCards)
        (if (Utilities|Array|ContainsItem (LocalVariables|GetHand) _array_element)
          (Class|UnicornCardActor|SetCanEnterStable _array_element true))))
    (:else)))

(fn DisableCards
  (bind _cardmanager (Variables|Default|GetCardManager)
    (:then
      (Utilities|Array|Clear (Variables|Default|GetListOfAffectedCards))
      (for _array_element (Class|UnicornCardGameManager|GetPlayerHand _cardmanager (Variables|Default|GetCurrentOwningPlayer))
        (if (Utilities|Enum|Equal(Enum) (.cardtype (Class|UnicornCardActor|GetCardInfo _array_element)) "Upgrade")
          (Utilities|Array|Add (Variables|Default|GetListOfAffectedCards) _array_element)
          (Class|UnicornCardActor|SetCanEnterStable _array_element false))))
    (:else)))