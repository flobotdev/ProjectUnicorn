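; Blinding Light is a downgrade card that blocks Magical Unicorn effects in the owning player's stable.
; On entering the stable it disables and records those unicorns, then listens for stable changes to rescan on additions and restore tracked cards that are removed.
; Leaving re-enables tracked cards still in the stable, though it unbinds from the hand-changed event rather than the stable-changed event it bound.
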(event Custom|OnPlayerStableChanged
  (params (PlayerIndex :type Integer) (Card :type Unicorn%20Card%20Actor%20Object%20Reference) (bRemoved :type Boolean))
  (if (== PlayerIndex (Variables|Default|GetCurrentOwningPlayer))
    (if bRemoved
      (if (Utilities|Array|ContainsItem (Variables|Default|GetList%20Of%20Affected%20Cards) Card)
        (Class|UnicornCardActor|SetCanPlayEffects Card true)
        (Utilities|Array|RemoveItem (Variables|Default|GetList%20Of%20Affected%20Cards) Card))
      (else
        (CallFunction|DisableCards)))))

(event EventOnLeaveStable
  (|CallParentFunction)
  (CallFunction|Revert)
  (EventDispatchers|UnbindEventfromOnPlayerHandChanged (Variables|Default|GetCardManager) (EventDispatchers|CreateEvent :!event Custom|OnPlayerStableChanged)))

(event EventOnEnterStable
  (CallFunction|DisableCards)
  (EventDispatchers|BindEventtoOnPlayerStableChanged (Variables|Default|GetCardManager) (EventDispatchers|CreateEvent :!event Custom|OnPlayerStableChanged)))

(fn ConstructionScript
  (|CallParentFunction))

(fn Revert
  (bind _cardmanager (Variables|Default|GetCardManager)
    (:then
      (LocalVariables|SetStable (Class|UnicornCardGameManager|GetPlayerStableUnicorns _cardmanager (Variables|Default|GetCurrentOwningPlayer)))
      (for _array_element (Variables|Default|GetList%20Of%20Affected%20Cards)
        (if (Utilities|Array|ContainsItem (LocalVariables|GetStable) _array_element)
          (Class|UnicornCardActor|SetCanPlayEffects _array_element true))))
    (:else)))

(fn DisableCards
  (bind _cardmanager (Variables|Default|GetCardManager)
    (:then
      (Utilities|Array|Clear (Variables|Default|GetList%20Of%20Affected%20Cards))
      (for _array_element (Class|UnicornCardGameManager|GetPlayerStableUnicorns _cardmanager (Variables|Default|GetCurrentOwningPlayer))
        (if (Utilities|Enum|Equal(Enum) (.cardtype (Class|UnicornCardActor|GetCardInfo _array_element)) "MagicalUnicorn")
          (Utilities|Array|Add (Variables|Default|GetList%20Of%20Affected%20Cards) _array_element)
          (Class|UnicornCardActor|SetCanPlayEffects _array_element false))))
    (:else)))