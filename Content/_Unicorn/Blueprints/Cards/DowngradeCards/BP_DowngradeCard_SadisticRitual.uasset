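; BP_DowngradeCard_SadisticRitual is a downgrade card that forces its owner to resolve the card's effect at phase start, then grants them a draw.
; OnBeginPhase invokes the mandatory effect through CardManager on the owner's turn and binds to its execution event, or completes the phase if invocation fails.
; When the matching effect executes, it gives the owner a draw-pile card, unbinds and completes the phase.
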(event Custom|OnEffectExecuted
  (params (Effect :type EEffectWord%20Enum :default "None") (PlayerIndex :type Integer) (bOptional :type Boolean))
  (if (Utilities|Enum|Equal(Enum) Effect (Utilities|Struct|BreakUnicornCardInfo (Variables|Default|GetCardInfo)))
    (Class|UnicornCardGameManager|GiveCardtoPlayerfromDrawPile (Variables|Default|GetCardManager) (Variables|Default|GetCurrentOwningPlayer))
    (EventDispatchers|UnbindEventfromOnEffectEventExecuted (Variables|Default|GetCardManager) (EventDispatchers|CreateEvent :!event Custom|OnEffectExecuted))
    (Default|CallOnCardPhaseCompleted (Variables|Default|GetCardManager))))

(fn ConstructionScript
  (|CallParentFunction))

(fn OnBeginPhase
  (bind _cardmanager (Variables|Default|GetCardManager)
    (:then
      (if (== (Class|UnicornCardGameManager|GetCurrentPlayerIndex _cardmanager) (Variables|Default|GetCurrentOwningPlayer))
        (bind _returnvalue (Class|UnicornCardGameManager|InvokeEffect (Variables|Default|GetCardManager) (Variables|Default|GetCurrentOwningPlayer) (Utilities|Struct|BreakUnicornCardInfo (Variables|Default|GetCardInfo)) false))
        (if _returnvalue
          (EventDispatchers|BindEventtoOnEffectEventExecuted (Variables|Default|GetCardManager) (EventDispatchers|CreateEvent :!event Custom|OnEffectExecuted))
          (else
            (Default|CallOnCardPhaseCompleted (Variables|Default|GetCardManager))
            (return true)))))
    (:else)))