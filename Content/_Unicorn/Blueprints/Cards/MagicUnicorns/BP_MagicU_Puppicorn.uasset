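; BP_MagicU_Puppicorn is the Puppicorn Magic Unicorn card, which moves itself between stables as turns begin.
; Its OnBeginPhase gets BP_Unicorn_GameMode and has the CardManager move the card to the current player's stable.
; The function returns true whether or not the cast succeeds, and the event graph holds only disabled default events.
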(event EventBeginPlay
  (|CallParentFunction) ; This node is disabled and will not be called.\nDrag off pins to build functionality.
)

(event Collision|EventActorBeginOverlap
  (params (OtherActor :type Actor%20Object%20Reference))
  (|CallParentFunction OtherActor) ; This node is disabled and will not be called.\nDrag off pins to build functionality.
)

(event EventTick
  (params (DeltaSeconds :type Float%20%28single-precision%29))
  (|CallParentFunction DeltaSeconds) ; This node is disabled and will not be called.\nDrag off pins to build functionality.
)

(fn ConstructionScript
  (|CallParentFunction))

(fn OnBeginPhase
  (bind _asbp_unicorn_game_mode (Utilities|Casting|CastToBP_Unicorn_GameMode (Game|GetGameMode))
    (:then
      (Class|UnicornCardGameManager|MovetoPlayerStable (Variables|/Game/_Unicorn/Blueprints/BP_Unicorn_GameMode.BP_Unicorn_GameMode_C|GetCardManager _asbp_unicorn_game_mode) (Class|UnicornCardGameManager|GetCurrentPlayerIndex (Variables|/Game/_Unicorn/Blueprints/BP_Unicorn_GameMode.BP_Unicorn_GameMode_C|GetCardManager _asbp_unicorn_game_mode)) self))
    (:CastFailed
      _))
  (return true))