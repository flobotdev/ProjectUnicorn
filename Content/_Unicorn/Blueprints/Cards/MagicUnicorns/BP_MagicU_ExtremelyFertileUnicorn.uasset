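; Magic Unicorn card "Extremely Fertile Unicorn", which offers its owner an optional effect to gain a Baby from the Nursery.
; On the owner's begin phase, OnBeginPhase invokes the effect through CardManager and, if that succeeds, binds executed and optional-ended events.
; Execution moves a random Nursery card to the current player's Stable.
; Both outcomes unbind the events and signal phase completion, as do failed checks immediately.
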(event Custom|OnEffectExecuted
  (params (Effect :type EEffectWord%20Enum :default "None") (PlayerIndex :type Integer) (bOptional :type Boolean))
  (if (Utilities|Enum|Equal(Enum) Effect (Utilities|Struct|BreakUnicornCardInfo (Variables|Default|GetCardInfo)))
    (CallFunction|GetBabyfromNursery)
    (Default|CallOnCardPhaseCompleted (Variables|Default|GetCardManager))
    (EventDispatchers|UnbindEventfromOnCardEffectOptionalEnded (Variables|Default|GetCardManager) (EventDispatchers|CreateEvent :!event Custom|OnCardEffectOptionalEnded))
    (EventDispatchers|UnbindEventfromOnEffectEventExecuted (Variables|Default|GetCardManager) (EventDispatchers|CreateEvent :!event Custom|OnEffectExecuted))))

(event Custom|OnCardEffectOptionalEnded
  (Default|CallOnCardPhaseCompleted (Variables|Default|GetCardManager))
  (EventDispatchers|UnbindEventfromOnCardEffectOptionalEnded (Variables|Default|GetCardManager) (EventDispatchers|CreateEvent :!event Custom|OnCardEffectOptionalEnded))
  (EventDispatchers|UnbindEventfromOnEffectEventExecuted (Variables|Default|GetCardManager) (EventDispatchers|CreateEvent :!event Custom|OnEffectExecuted)))

(fn ConstructionScript
  (|CallParentFunction))

(fn GetBabyfromNursery
  (bind _cardmanager (Variables|Default|GetCardManager)
    (:then
      (LocalVariables|SetBaby (.OutItem (Utilities|Array|Random (Class|UnicornCardGameManager|GetNursery _cardmanager))))
      (Class|UnicornCardGameManager|RemovefromNursery _cardmanager (LocalVariables|GetBaby))
      (Class|UnicornCardGameManager|AddtoPlayerStable _cardmanager (Class|UnicornCardGameManager|GetCurrentPlayerIndex _cardmanager) (LocalVariables|GetBaby)))
    (:else)))

(fn OnBeginPhase
  (Variables|Default|GetCardManager
    (:then
      (if (== (Class|UnicornCardGameManager|GetCurrentPlayerIndex (Variables|Default|GetCardManager)) (Variables|Default|GetCurrentOwningPlayer))
        (bind _returnvalue (Class|UnicornCardActor|CanPlayEffects))
        (if _returnvalue
          (bind _returnvalue_2 (Class|UnicornCardGameManager|InvokeEffect (Variables|Default|GetCardManager) (Variables|Default|GetCurrentOwningPlayer) (Utilities|Struct|BreakUnicornCardInfo (Variables|Default|GetCardInfo)) true))
          (if _returnvalue_2
            (EventDispatchers|BindEventtoOnEffectEventExecuted (Variables|Default|GetCardManager) (EventDispatchers|CreateEvent :!event Custom|OnEffectExecuted))
            (EventDispatchers|BindEventtoOnCardEffectOptionalEnded (Variables|Default|GetCardManager) (EventDispatchers|CreateEvent :!event Custom|OnCardEffectOptionalEnded))
            (return false)
            (else
              _)))))
    (:else
      _))
  (Default|CallOnCardPhaseCompleted (Variables|Default|GetCardManager))
  (return true))