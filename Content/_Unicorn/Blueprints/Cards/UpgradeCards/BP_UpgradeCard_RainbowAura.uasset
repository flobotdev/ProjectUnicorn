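; Rainbow Aura upgrade card that makes the owning player's Basic, Magical and Baby Unicorns indestructible while it is in their stable.
; DisableCards clears its tracking list, then records and protects destroyable unicorns, rerunning on additions, so earlier protected cards drop off the list.
; Removed cards and Revert on leave restore only tracked cards.
; Leaving unbinds from hand changes, although entering binds to stable changes.
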(event Custom|OnPlayerStableChanged
  (params (PlayerIndex :type Integer) (Card :type Unicorn%20Card%20Actor%20Object%20Reference) (bRemoved :type Boolean))
  (if (== PlayerIndex (Variables|Default|GetCurrentOwningPlayer))
    (if bRemoved
      (if (Utilities|Array|ContainsItem (Variables|Default|GetList%20Of%20Affected%20Cards) Card)
        (Variables|/Script/ProjectUnicorn.UnicornCardActor|SetbCanBeDestroyed Card true)
        (Utilities|Array|RemoveItem (Variables|Default|GetList%20Of%20Affected%20Cards) Card))
      (else
        (CallFunction|DisableCards)))))

(event EventOnEnterStable
  (|CallParentFunction)
  (CallFunction|DisableCards)
  (EventDispatchers|BindEventtoOnPlayerStableChanged (Variables|Default|GetCardManager) (EventDispatchers|CreateEvent :!event Custom|OnPlayerStableChanged)))

(event EventOnLeaveStable
  (|CallParentFunction)
  (CallFunction|Revert)
  (EventDispatchers|UnbindEventfromOnPlayerHandChanged (Variables|Default|GetCardManager) (EventDispatchers|CreateEvent :!event Custom|OnPlayerStableChanged)))

(fn ConstructionScript
  (|CallParentFunction))

(fn DisableCards
  (bind _cardmanager (Variables|Default|GetCardManager)
    (:then
      (Utilities|Array|Clear (Variables|Default|GetList%20Of%20Affected%20Cards))
      (for _array_element (Class|UnicornCardGameManager|GetPlayerStableUnicorns _cardmanager (Variables|Default|GetCurrentOwningPlayer))
        (switch Utilities|FlowControl|Switch|SwitchonECardType (.cardtype (Class|UnicornCardActor|GetCardInfo _array_element))
          (:MagicalUnicorn
            _)
          (:BasicUnicorn
            _)
          (:BabyUnicorn
            _))
        (if (Variables|/Script/ProjectUnicorn.UnicornCardActor|GetbCanBeDestroyed _array_element)
          (Utilities|Array|Add (Variables|Default|GetList%20Of%20Affected%20Cards) _array_element)
          (Variables|/Script/ProjectUnicorn.UnicornCardActor|SetbCanBeDestroyed _array_element false))))
    (:else)))

(fn Revert
  (bind _cardmanager (Variables|Default|GetCardManager)
    (:then
      (LocalVariables|SetStable (Class|UnicornCardGameManager|GetPlayerStableUnicorns _cardmanager (Variables|Default|GetCurrentOwningPlayer)))
      (for _array_element (Variables|Default|GetList%20Of%20Affected%20Cards)
        (if (Utilities|Array|ContainsItem (LocalVariables|GetStable) _array_element)
          (Variables|/Script/ProjectUnicorn.UnicornCardActor|SetbCanBeDestroyed _array_element true))))
    (:else)))