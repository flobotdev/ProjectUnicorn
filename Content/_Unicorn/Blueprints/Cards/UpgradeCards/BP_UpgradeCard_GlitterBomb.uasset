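; Glitter Bomb upgrade card that gives its owner an optional effect at the start of a phase, followed by a Destroy effect.
; OnBeginPhase invokes the card's own effect through CardManager and listens for its result, completing immediately for other players or failed invokes.
; Executing that effect triggers a mandatory Destroy; a Destroy execution or optional end completes the phase and unbinds.
; CanPlayCard also requires Destroy to be invokable.
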(event Custom|OnOptionalEndTurn
  (Default|CallOnCardPhaseCompleted (Variables|Default|GetCardManager))
  (EventDispatchers|UnbindEventfromOnCardEffectOptionalEnded (Variables|Default|GetCardManager) (EventDispatchers|CreateEvent :!event Custom|OnOptionalEndTurn))
  (EventDispatchers|UnbindEventfromOnEffectEventExecuted (Variables|Default|GetCardManager) (EventDispatchers|CreateEvent :!event Custom|OnEffectExecuted)))

(event Custom|OnEffectExecuted
  (params (Effect :type EEffectWord%20Enum :default "None") (PlayerIndex :type Integer) (bOptional :type Boolean))
  (if (and (== PlayerIndex (Variables|Default|GetCurrentOwningPlayer)) (Utilities|Enum|Equal(Enum) Effect (Utilities|Struct|BreakUnicornCardInfo (Variables|Default|GetCardInfo))))
    (Class|UnicornCardGameManager|InvokeEffect (Variables|Default|GetCardManager) (Variables|Default|GetCurrentOwningPlayer) "Destroy" false)
    (elif (Utilities|Enum|Equal(Enum) Effect "Destroy")
      (Default|CallOnCardPhaseCompleted (Variables|Default|GetCardManager))
      (EventDispatchers|UnbindEventfromOnCardEffectOptionalEnded (Variables|Default|GetCardManager) (EventDispatchers|CreateEvent :!event Custom|OnOptionalEndTurn))
      (EventDispatchers|UnbindEventfromOnEffectEventExecuted (Variables|Default|GetCardManager) (EventDispatchers|CreateEvent :!event Custom|OnEffectExecuted)))))

(event EventBeginPlay
  (|CallParentFunction) ; This node is disabled and will not be called.\nDrag off pins to build functionality.
)

(event Collision|EventActorBeginOverlap
  (params (OtherActor :type Actor%20Object%20Reference))
  (|CallParentFunction OtherActor) ; This node is disabled and will not be called.\nDrag off pins to build functionality.
)

(event EventTick
  (params (DeltaSeconds :type Float%20%28single-precision%29))
  (|CallParentFunction DeltaSeconds) ; This node is disabled and will not be called.\nDrag off pins to build functionality.
)

(fn ConstructionScript
  (|CallParentFunction))

(fn OnBeginPhase
  (if (== (Class|UnicornCardGameManager|GetCurrentPlayerIndex (Variables|Default|GetCardManager)) (Variables|Default|GetCurrentOwningPlayer))
    (bind _returnvalue (Class|UnicornCardGameManager|InvokeEffect (Variables|Default|GetCardManager) (Variables|Default|GetCurrentOwningPlayer) (Utilities|Struct|BreakUnicornCardInfo (Variables|Default|GetCardInfo)) true))
    (if _returnvalue
      (EventDispatchers|BindEventtoOnEffectEventExecuted (Variables|Default|GetCardManager) (EventDispatchers|CreateEvent :!event Custom|OnEffectExecuted))
      (EventDispatchers|BindEventtoOnCardEffectOptionalEnded (Variables|Default|GetCardManager) (EventDispatchers|CreateEvent :!event Custom|OnOptionalEndTurn))
      (return false)
      (else
        _)))
  (Default|CallOnCardPhaseCompleted (Variables|Default|GetCardManager))
  (return true))

(fn CanPlayCard
  (bind _returnvalue (|CallParentFunction))
  (bind _returnvalue_2 (Class|UnicornCardGameManager|CanInvokeEffect (Variables|Default|GetCardManager) (Variables|Default|GetCurrentOwningPlayer) "Destroy"))
  (return (and _returnvalue_2 _returnvalue)))