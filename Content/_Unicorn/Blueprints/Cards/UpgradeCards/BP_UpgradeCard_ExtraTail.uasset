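; Extra Tail upgrade card, which gives its owner an extra card from the draw pile at the start of their turn.
; It can only enter a stable that holds at least one Basic Unicorn, checked through the CardManager.
; On begin phase it draws only when the owner is the current player, then always notifies the CardManager that the card phase is complete.
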(event EventBeginPlay
  (|CallParentFunction) ; This node is disabled and will not be called.\nDrag off pins to build functionality.
)

(event Collision|EventActorBeginOverlap
  (params (OtherActor :type Actor%20Object%20Reference))
  (|CallParentFunction OtherActor) ; This node is disabled and will not be called.\nDrag off pins to build functionality.
)

(event EventTick
  (params (DeltaSeconds :type Float%20%28single-precision%29))
  (|CallParentFunction DeltaSeconds) ; This node is disabled and will not be called.\nDrag off pins to build functionality.
)

(fn ConstructionScript
  (|CallParentFunction))

(fn CanEnterStable
  (bind _array_element (Utilities|Array|ForEachLoopwithBreak (Class|UnicornCardGameManager|GetPlayerStableUnicorns (Variables|Default|GetCardManager) (Variables|Default|GetCurrentOwningPlayer)))
    (:LoopBody
      (switch Utilities|FlowControl|Switch|SwitchonECardType (.CardType (Utilities|Struct|BreakUnicornCardInfo (Class|UnicornCardActor|GetCardInfo _array_element)))
        (:BasicUnicorn
          (return true))))
    (:Completed
      (return false))))

(fn OnBeginPhase
  (if (== (Class|UnicornCardGameManager|GetCurrentPlayerIndex (Variables|Default|GetCardManager)) (Variables|Default|GetCurrentOwningPlayer))
    (Class|UnicornCardGameManager|GiveCardtoPlayerfromDrawPile (Variables|Default|GetCardManager) (Variables|Default|GetCurrentOwningPlayer)))
  (Default|CallOnCardPhaseCompleted (Variables|Default|GetCardManager))
  (return true))