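; Unicorn Lasso upgrade card that lets its owner optionally steal a card at the start of their turn and gives it back when the phase ends.
; At begin phase it invokes an optional Steal through CardManager and binds events to record the card entering the owner's stable and the effect's player index.
; At end phase, a completed steal moves that card to the recorded player's stable and clears the saved state.
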(event Custom|OnEffectExecuted
  (params (Effect :type EEffectWord%20Enum :default "None") (PlayerIndex :type Integer) (bOptional :type Boolean))
  (if (Utilities|Enum|Equal(Enum) Effect "Steal")
    (Development|PrintString (Utilities|String|ToString(Integer) PlayerIndex))
    (EventDispatchers|UnbindEventfromOnEffectEventExecuted (Variables|Default|GetCardManager) (EventDispatchers|CreateEvent :!event Custom|OnEffectExecuted))
    (Variables|Default|SetPlayer%20Index PlayerIndex)
    (Variables|Default|SetReturnCard true)
    (Default|CallOnCardPhaseCompleted (Variables|Default|GetCardManager))))

(event Custom|OnPlayerStableChanged
  (params (PlayerIndex :type Integer) (Card :type Unicorn%20Card%20Actor%20Object%20Reference) (bRemoved :type Boolean))
  (if (and (== PlayerIndex (Variables|Default|GetCurrentOwningPlayer)) (not bRemoved))
    (EventDispatchers|UnbindEventfromOnPlayerStableChanged (Variables|Default|GetCardManager) (EventDispatchers|CreateEvent :!event Custom|OnPlayerStableChanged))
    (Variables|Default|SetCard Card)))

(event Custom|OnOptionalEnded
  (EventDispatchers|UnbindEventfromOnEffectEventExecuted (Variables|Default|GetCardManager) (EventDispatchers|CreateEvent :!event Custom|OnEffectExecuted))
  (EventDispatchers|UnbindEventfromOnPlayerStableChanged (Variables|Default|GetCardManager) (EventDispatchers|CreateEvent :!event Custom|OnPlayerStableChanged))
  (Default|CallOnCardPhaseCompleted (Variables|Default|GetCardManager)))

(fn ConstructionScript
  (|CallParentFunction))

(fn OnBeginPhase
  (if (== (Class|UnicornCardGameManager|GetCurrentPlayerIndex (Variables|Default|GetCardManager)) (Variables|Default|GetCurrentOwningPlayer))
    (bind _returnvalue (Class|UnicornCardGameManager|InvokeEffect (Variables|Default|GetCardManager) (Variables|Default|GetCurrentOwningPlayer) "Steal" true))
    (if _returnvalue
      (EventDispatchers|BindEventtoOnCardEffectOptionalEnded (Variables|Default|GetCardManager) (EventDispatchers|CreateEvent :!event Custom|OnOptionalEnded))
      (EventDispatchers|BindEventtoOnPlayerStableChanged (Variables|Default|GetCardManager) (EventDispatchers|CreateEvent :!event Custom|OnPlayerStableChanged))
      (EventDispatchers|BindEventtoOnEffectEventExecuted (Variables|Default|GetCardManager) (EventDispatchers|CreateEvent :!event Custom|OnEffectExecuted))
      (else
        (Default|CallOnCardPhaseCompleted (Variables|Default|GetCardManager) :!label _label)))
    (else
      (goto _label)))
  (return true))

(fn OnEndPhase
  (if (Variables|Default|GetReturnCard)
    (Class|UnicornCardGameManager|MovetoPlayerStable (Variables|Default|GetCardManager) (Variables|Default|GetPlayer%20Index) (Variables|Default|GetCard))
    (Variables|Default|SetCard 0)
    (Variables|Default|SetPlayer%20Index -1)
    (Variables|Default|SetReturnCard false))
  (Default|CallOnCardPhaseCompleted (Variables|Default|GetCardManager))
  (return true))