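; BP_MagicCard_UnicornPoison is the Unicorn Poison magic card, which triggers a mandatory Destroy effect for the player who owns it when played.
; OnPlayedCard runs the parent logic, invokes the effect through CardManager, then binds to its effect-executed event.
; When that event reports a Destroy, the card tells CardManager to advance to the next phase.
; A TODO notes that having no destroyable cards is unhandled.
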(event Custom|OnEffectExecuted
  (params (Effect :type EEffectWord%20Enum :default "None") (PlayerIndex :type Integer) (bOptional :type Boolean))
  (if (Utilities|Enum|Equal(Enum) Effect "Destroy")
    (Class|UnicornCardGameManager|NextPhase (Variables|Default|GetCardManager))))

(event EventBeginPlay
  (|CallParentFunction) ; This node is disabled and will not be called.\nDrag off pins to build functionality.
)

(event Collision|EventActorBeginOverlap
  (params (OtherActor :type Actor%20Object%20Reference))
  (|CallParentFunction OtherActor) ; This node is disabled and will not be called.\nDrag off pins to build functionality.
)

(event EventTick
  (params (DeltaSeconds :type Float%20%28single-precision%29))
  (|CallParentFunction DeltaSeconds) ; This node is disabled and will not be called.\nDrag off pins to build functionality.
)

(event EventOnPlayedCard
  (|CallParentFunction)
  (Variables|Default|GetCardManager
    (:then
      ;[0.15 0.15 0.15 0.5] TODO: what if there's no destroyable cards? handle it
      (Class|UnicornCardGameManager|InvokeEffect (Variables|Default|GetCardManager) (Variables|Default|GetCurrentOwningPlayer) "Destroy" false)
      (EventDispatchers|BindEventtoOnEffectEventExecuted (Variables|Default|GetCardManager) (EventDispatchers|CreateEvent :!event Custom|OnEffectExecuted)))
    (:else)))

(fn ConstructionScript
  (|CallParentFunction))