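; Magic card Blueprint for Kick Back, which chains a Revert effect into a forced Discard for the affected player.
; When played, it triggers a mandatory Revert for the current player through the game mode's CardManager.
; One-shot event bindings sequence the steps: the next stable change selects who must discard, and that player's hand removal ends listening.
; A NextPhase call is present but disconnected.
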(event Custom|OnPlayerStableChanged
  (params (PlayerIndex :type Integer) (Card :type Unicorn%20Card%20Actor%20Object%20Reference) (bRemoved :type Boolean))
  (EventDispatchers|UnbindEventfromOnPlayerStableChanged (Variables|Default|GetCard%20Manager) (EventDispatchers|CreateEvent :!event Custom|OnPlayerStableChanged))
  (Variables|Default|SetTargetPlayer PlayerIndex)
  (Default|CallOnEffectCard (Variables|Default|GetCard%20Manager) PlayerIndex "Discard" false)
  (EventDispatchers|BindEventtoOnPlayerHandChanged (Variables|Default|GetCard%20Manager) (EventDispatchers|CreateEvent :!event Custom|OnPlayerHandChanged)))

(event Custom|OnPlayerHandChanged
  (params (PlayerIndex :type Integer) (Card :type Unicorn%20Card%20Actor%20Object%20Reference) (bRemoved :type Boolean))
  (if (and (== (Variables|Default|GetTargetPlayer) PlayerIndex) bRemoved)
    (EventDispatchers|UnbindEventfromOnPlayerHandChanged (Variables|Default|GetCard%20Manager) (EventDispatchers|CreateEvent :!event Custom|OnPlayerHandChanged))))

(event EventBeginPlay
  (|CallParentFunction) ; This node is disabled and will not be called.\nDrag off pins to build functionality.
)

(event Collision|EventActorBeginOverlap
  (params (OtherActor :type Actor%20Object%20Reference))
  (|CallParentFunction OtherActor) ; This node is disabled and will not be called.\nDrag off pins to build functionality.
)

(event EventTick
  (params (DeltaSeconds :type Float%20%28single-precision%29))
  (|CallParentFunction DeltaSeconds) ; This node is disabled and will not be called.\nDrag off pins to build functionality.
)

(event EventOnPlayedCard
  (|CallParentFunction)
  (bind _asbp_unicorn_game_mode (Utilities|Casting|CastToBP_Unicorn_GameMode (Game|GetGameMode)))
  (Variables|Default|SetCard%20Manager (Variables|/Game/_Unicorn/Blueprints/BP_Unicorn_GameMode.BP_Unicorn_GameMode_C|GetCardManager _asbp_unicorn_game_mode))
  (Default|CallOnEffectCard (Variables|Default|GetCard%20Manager) (Class|UnicornCardGameManager|GetCurrentPlayerIndex (Variables|Default|GetCard%20Manager)) "Revert" false)
  (EventDispatchers|BindEventtoOnPlayerStableChanged (Variables|Default|GetCard%20Manager) (EventDispatchers|CreateEvent :!event Custom|OnPlayerStableChanged)))

(fn ConstructionScript
  (|CallParentFunction))